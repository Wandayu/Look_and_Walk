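; BP_TableIndicator is a marker actor that highlights one of four tables, A to D.
; It starts hidden, with collision disabled on its Plane.
; ShowAtTable switches on the table enum, teleports the root to a hard-coded world position for that table and unhides it with its children.
; Hide conceals it again.
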(event Custom|ShowAtTable
  (params (Table :type String))
  (switch string Table
    (:A
      (Transformation|SetWorldLocation (Variables|Default|GetDefaultSceneRoot) "95.000000,515.000000,103.000000" false true))
    (:B
      (Transformation|SetWorldLocation (Variables|Default|GetDefaultSceneRoot) "95.000000,325.000000,103.000000" false true))
    (:C
      (Transformation|SetWorldLocation (Variables|Default|GetDefaultSceneRoot) "95.000000,135.000000,103.000000" false true))
    (:D
      (Transformation|SetWorldLocation (Variables|Default|GetDefaultSceneRoot) "95.000000,-55.000000,103.000000" false true)))
  (Development|SetHiddeninGame (Variables|Default|GetDefaultSceneRoot) false true))

(event Custom|Hide
  (Development|SetHiddeninGame (Variables|Default|GetDefaultSceneRoot) true true))

(event EventBeginPlay
  (Development|SetHiddeninGame (Variables|Default|GetDefaultSceneRoot) true true)
  (Collision|SetCollisionEnabled (Variables|Default|GetPlane) "NoCollision"))

(event Collision|EventActorBeginOverlap
  (params (OtherActor :type Actor%20Object%20Reference)))

(event EventTick
  (params (DeltaSeconds :type Float%20%28single-precision%29)))

(fn ConstructionScript)