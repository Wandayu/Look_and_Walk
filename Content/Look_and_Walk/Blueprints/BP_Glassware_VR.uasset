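; VR lab glassware actor whose liquid drains when tipped, refills from other glassware and blends colours.
; Construction picks the mesh by glassware type and creates a dynamic material for liquid amount, colour and position.
; Tick treats a cap below the mesh origin as pouring, toggling a looping drain timer, and pushes world position to work around a grab bug.
; Cap-to-cap overlaps while upright toggle the fill timer and start a timeline blending halfway toward the other liquid's colour.
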(event OnComponentBeginOverlap(Collision_Cap)
  (params (OverlappedComponent :type Primitive%20Component%20Object%20Reference) (OtherActor :type Actor%20Object%20Reference) (OtherComp :type Primitive%20Component%20Object%20Reference) (OtherBodyIndex :type Integer) (bFromSweep :type Boolean) (SweepResult :type Hit%20Result%20Structure%20%28by%20ref%29))
  (bind _liquidamountincreasehandle (Variables|Default|GetLiquidAmountIncreaseHandle))
  (bind _liquid_colour (Variables|Default|GetLiquid%20Colour))
  ;[1 1 1] Get liquid from another bottle
  (bind _asbp_glassware_vr (Utilities|Casting|CastToBP_Glassware_VR OtherActor))
  (if (== (Variables|BP_Glassware_VR_C|GetCollision_Cap _asbp_glassware_vr) OtherComp)
    (if (not (CallFunction|IfPouringLiquid))
      ;[1 1 1] Record the glass
      (bind _output_get (Variables|Default|SetReceiveGlass _asbp_glassware_vr))
      (if (> (Variables|BP_Glassware_VR_C|GetLiquid%20Amount _output_get) 0.0)
        (Utilities|Array|Add (Variables|Default|GetReceiveGlassList) (Utilities|GetDisplayName _output_get))
        ;[1 1 1] Start to increase
        (if (Class|KismetSystemLibrary|IsTimerPausedHandle _liquidamountincreasehandle)
          (Utilities|Time|UnpauseTimerbyHandle _liquidamountincreasehandle)
          ;[1 1 1] Mix the color of two liquid
          (bind _alpha (Timeline|MixColorCurve PlayFromStart)
            (:Update
              (Rendering|Material|SetVectorParameterValue (Variables|Default|GetGlasswareMaterial) "Liquid Colour" (Math|Color|Lerp(LinearColor) _liquid_colour (Math|Color|Lerp(LinearColor) _liquid_colour (Variables|BP_Glassware_VR_C|GetLiquid%20Colour _asbp_glassware_vr) 0.5) _alpha) :!class /Script/Engine.MaterialInstanceDynamic))))
        (else
          (Utilities|Time|PauseTimerbyHandle (Variables|Default|GetLiquidAmountIncreaseHandle)))))))

(event OnComponentEndOverlap(Collision_Cap)
  (params (OverlappedComponent :type Primitive%20Component%20Object%20Reference) (OtherActor :type Actor%20Object%20Reference) (OtherComp :type Primitive%20Component%20Object%20Reference) (OtherBodyIndex :type Integer))
  (bind _liquidamountincreasehandle (Variables|Default|GetLiquidAmountIncreaseHandle))
  ;[1 1 1] Get liquid from another bottle
  (bind _asbp_glassware_vr (Utilities|Casting|CastToBP_Glassware_VR OtherActor))
  (if (== (Variables|BP_Glassware_VR_C|GetCollision_Cap _asbp_glassware_vr) OtherComp)
    (if (not (CallFunction|IfPouringLiquid))
      ;[1 1 1] Stop to increase
      (if (not (Class|KismetSystemLibrary|IsTimerPausedHandle _liquidamountincreasehandle))
        (Utilities|Time|PauseTimerbyHandle _liquidamountincreasehandle)
        ;[1 1 1] Record the current color
        (bind _returnvalue (Rendering|Material|GetVectorParameterValue (Variables|Default|GetGlasswareMaterial) "Liquid Colour" :!class /Script/Engine.MaterialInstanceDynamic))
        (Variables|Default|SetLiquid%20Colour _returnvalue)))))

(event Custom|LiquidAmountDecrease
  (if (> (Variables|Default|GetLiquid%20Amount) 0.0)
    (Variables|Default|SetLiquid%20Amount (- (Variables|Default|GetLiquid%20Amount) 0.1))
    (Rendering|Material|SetScalarParameterValue (Variables|Default|GetGlasswareMaterial) "Liquid Amount" (Variables|Default|GetLiquid%20Amount) :!class /Script/Engine.MaterialInstanceDynamic)))

(event Custom|LiquidAmountIncrease
  (if (and (< (Variables|Default|GetLiquid%20Amount) 1.0) (> (Variables|BP_Glassware_VR_C|GetLiquid%20Amount (Variables|Default|GetReceiveGlass)) 0.0))
    (Variables|Default|SetLiquid%20Amount (+ (Variables|Default|GetLiquid%20Amount) 0.005))
    (Rendering|Material|SetScalarParameterValue (Variables|Default|GetGlasswareMaterial) "Liquid Amount" (Variables|Default|GetLiquid%20Amount) :!class /Script/Engine.MaterialInstanceDynamic)))

(event EventBeginPlay
  (bind _returnvalue (Utilities|Time|SetTimerbyEvent (delegate Custom|LiquidAmountDecrease) 0.2 true))
  (bind _output_get (Variables|Default|SetLiquidAmoundDecreaseHandle _returnvalue))
  (Utilities|Time|PauseTimerbyHandle _output_get)
  (bind _returnvalue_2 (Utilities|Time|SetTimerbyEvent (delegate Custom|LiquidAmountIncrease) 0.1 true))
  (bind _output_get_2 (Variables|Default|SetLiquidAmountIncreaseHandle _returnvalue_2))
  (Utilities|Time|PauseTimerbyHandle _output_get_2))

(event Collision|EventActorBeginOverlap
  (params (OtherActor :type Actor%20Object%20Reference)))

(event EventTick
  (params (DeltaSeconds :type Float%20%28single-precision%29))
  (bind _liquidamounddecreasehandle (Variables|Default|GetLiquidAmoundDecreaseHandle))
  (bind _liquidamounddecreasehandle_2 (Variables|Default|GetLiquidAmoundDecreaseHandle))
  (bind _returnvalue (Class|KismetSystemLibrary|IsTimerPausedHandle _liquidamounddecreasehandle))
  ;[1 0 0.04338] Actor position in shader will give the hand position when grabbing rather than object's position, so update manually (This is Unreal's Bug!!!)
  (Rendering|Material|SetVectorParameterValue (Variables|Default|GetGlasswareMaterial) "Position" (Math|Conversions|ToLinearColor(Vector) (Transformation|GetWorldLocation (Variables|Default|GetStaticMeshComponent))) :!class /Script/Engine.MaterialInstanceDynamic)
  (if (CallFunction|IfPouringLiquid)
    ;[1 1 1] (Stop) pour the liquid by (un)pausing the handle
    (if _returnvalue
      (Utilities|Time|UnpauseTimerbyHandle _liquidamounddecreasehandle_2))
    (elif (not _returnvalue)
      (Utilities|Time|PauseTimerbyHandle _liquidamounddecreasehandle_2))))

(fn ConstructionScript
  (|CallParentFunction)
  (Components|StaticMesh|SetStaticMesh (Variables|Default|GetStaticMeshComponent) (CallFunction|EGlasswareTypetoSM (Variables|Default|GetGlassware%20Type)))
  (bind _returnvalue (Rendering|Material|CreateDynamicMaterialInstance (Variables|Default|GetStaticMeshComponent) 0 0 "None" :!class /Script/Engine.PrimitiveComponent))
  (Variables|Default|SetGlasswareMaterial _returnvalue)
  (Rendering|Material|SetVectorParameterValue (Variables|Default|GetGlasswareMaterial) "Liquid Colour" (Variables|Default|GetLiquid%20Colour) :!class /Script/Engine.MaterialInstanceDynamic)
  (Rendering|Material|SetScalarParameterValue (Variables|Default|GetGlasswareMaterial) "Liquid Amount" (Variables|Default|GetLiquid%20Amount) :!class /Script/Engine.MaterialInstanceDynamic)
  (Rendering|Material|SetVectorParameterValue (Variables|Default|GetGlasswareMaterial) "Position" (Math|Conversions|ToLinearColor(Vector) (Transformation|GetWorldLocation (Variables|Default|GetStaticMeshComponent))) :!class /Script/Engine.MaterialInstanceDynamic))

(fn EGlasswareTypetoSM
  (params (Type :type E_Glassware_Type%20Enum :default "NewEnumerator0"))
  (return (Utilities|Select :Index Type :NewEnumerator0 "/Game/Laboratory_Equipment/Meshes/Beaker_500ml.Beaker_500ml" :NewEnumerator1 "/Game/Laboratory_Equipment/Meshes/Beaker_250ml.Beaker_250ml" :NewEnumerator2 "/Game/Laboratory_Equipment/Meshes/Conical_Flask_500ml.Conical_Flask_500ml" :NewEnumerator3 "/Game/Laboratory_Equipment/Meshes/Conical_Flask_250ml.Conical_Flask_250ml" :NewEnumerator4 "/Game/Laboratory_Equipment/Meshes/Flask1.Flask1" :NewEnumerator5 "/Game/Laboratory_Equipment/Meshes/Flask2.Flask2" :NewEnumerator13 "/Game/Laboratory_Equipment/Meshes/Tissue_Culture_Flask.Tissue_Culture_Flask" :NewEnumerator14 "/Game/Laboratory_Equipment/Meshes/Tissue_Culture_Flask_Base.Tissue_Culture_Flask_Base" :NewEnumerator6 "/Game/Laboratory_Equipment/Meshes/Graduated_Cylinder.Graduated_Cylinder" :NewEnumerator12 "/Game/Laboratory_Equipment/Meshes/Test_Tube.Test_Tube" :NewEnumerator11 "/Game/Laboratory_Equipment/Meshes/Petri_Dish.Petri_Dish" :NewEnumerator7 "/Game/Laboratory_Equipment/Meshes/Helix_Connecor_1.Helix_Connecor_1" :NewEnumerator8 "/Game/Laboratory_Equipment/Meshes/Helix_Connector_2.Helix_Connector_2" :NewEnumerator9 "/Game/Laboratory_Equipment/Meshes/Glass_Connecor_1.Glass_Connecor_1" :NewEnumerator10 "/Game/Laboratory_Equipment/Meshes/Glass_Connecor_2.Glass_Connecor_2")))

(fn SetLiquidColour
  (Variables|Default|SetLiquid%20Colour (CallFunction|GetColour))
  (Rendering|Material|SetVectorParameterValue (Variables|Default|GetGlasswareMaterial) "Liquid Colour" (Variables|Default|GetLiquid%20Colour) :!class /Script/Engine.MaterialInstanceDynamic))

(fn GetColour
  (return (Utilities|Select :Index (Math|Random|RandomIntegerinRange 0 11) :Option%200 "(R=0.000000,G=1.000000,B=0.000000,A=1.000000)" :Option%201 "(R=1.000000,G=0.000000,B=0.000000,A=1.000000)" :Option%202 "(R=0.000000,G=0.000000,B=1.000000,A=1.000000)" :Option%203 "(R=1.000000,G=1.000000,B=0.000000,A=1.000000)" :Option%204 "(R=0.700000,G=0.700000,B=0.700000,A=1.000000)" :Option%205 "(R=0.021219,G=0.078187,B=0.000000,A=1.000000)" :Option%206 "(R=0.372000,G=0.000000,B=0.500000,A=1.000000)" :Option%207 "(R=1.000000,G=0.100000,B=0.000000,A=1.000000)" :Option%208 "(R=0.000000,G=1.000000,B=1.000000,A=1.000000)" :Option%209 "(R=1.000000,G=0.000000,B=0.736000,A=1.000000)" :Option%2010 "(R=0.000000,G=0.000000,B=0.000000,A=1.000000)")))

(fn IfPouringLiquid
  (return (< (.z (Transformation|GetWorldLocation (Variables|Default|GetCollision_Cap))) (.z (Transformation|GetWorldLocation (Variables|Default|GetStaticMeshComponent))))))