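; BP_DataCollectionManager logs study data from a VR locomotion task to files under the game content directory.
; On BeginPlay it creates four files for task times, virtual positions, tracking-space positions and teleports, printing a warning if one exists.
; Looping timers accumulate global and per-step time and sample character and tracked-device positions between start and stop calls.
; Step durations are appended when timing ends, and teleports are logged with global time, start and destination.
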(event Custom|RecordGlobalTime
  ;[0.3277 1 0.2491] Record global testing time for record the teleport action
  (Variables|Default|SetGlobalRecordTime (+ (Variables|Default|GetGlobalRecordTime) (Variables|DataCollection|GetRecordTimeInterval))))

(event Custom|RecordTeleport
  (params (StartLocation :type Vector) (Destination :type Vector))
  (bind _spacestring (Variables|Default|GetSpaceString))
  (Class|EFMFile|AppendString (Variables|Default|GetTeleportLogFile) (Utilities|String|Append (Class|KismetStringLibrary|TimeSecondstoString (Variables|Default|GetGlobalRecordTime)) _spacestring (Utilities|String|ToString(Vector) StartLocation) _spacestring (Utilities|String|ToString(Vector) Destination))))

(event Custom|StartRecordPosition
  (Utilities|Time|SetTimerbyFunctionName self "RecordPosition" (Variables|DataCollection|GetRecordPositionInterval) true))

(event Custom|EndRecordPosition
  (Utilities|Time|ClearTimerbyFunctionName self "RecordPosition"))

(event EventBeginPlay
  ;[1 0.9216 0.07843] Create data collection files
  (bind _file (CallFunction|CreateFile (Variables|DataCollection|GetTaskTimeFileName)))
  (Variables|Default|SetTaskTimeFile _file)
  (bind _file_2 (CallFunction|CreateFile (Variables|DataCollection|GetVirtualPositionFileName)))
  (Variables|Default|SetVirtualPositionFile _file_2)
  (bind _file_3 (CallFunction|CreateFile (Variables|DataCollection|GetTrackingPositionFileName)))
  (Variables|Default|SetTrackingPositionFile _file_3)
  (bind _file_4 (CallFunction|CreateFile (Variables|DataCollection|GetTeleportLogFileName)))
  (Variables|Default|SetTeleportLogFile _file_4)
  ;[0.3277 1 0.2491] Record global testing time for record the teleport action
  (Utilities|Time|SetTimerbyEvent (delegate Custom|RecordGlobalTime) (Variables|DataCollection|GetRecordTimeInterval) true))

(event Collision|EventActorBeginOverlap
  (params (OtherActor :type Actor%20Object%20Reference)))

(event EventTick
  (params (DeltaSeconds :type Float%20%28single-precision%29)))

(fn ConstructionScript)

(fn StartRecordTime
  (Variables|Default|SetCurrentRecordTime 0.0)
  (Utilities|Time|SetTimerbyFunctionName self "RecordTime" (Variables|DataCollection|GetRecordTimeInterval) true))

(fn EndRecordTime
  (params (CurrentStep :type String))
  (Utilities|Time|ClearTimerbyFunctionName self "RecordTime")
  ;[1 1 1] Record time to finish the task
  (Class|EFMFile|AppendString (Variables|Default|GetTaskTimeFile) (Utilities|String|Append (Utilities|String|Append CurrentStep (Variables|Default|GetSpaceString)) (Utilities|String|ToString(Float) (Variables|Default|GetCurrentRecordTime))))
  (Variables|Default|SetCurrentRecordTime 0.0))

(fn RecordTime
  (Variables|Default|SetCurrentRecordTime (+ (Variables|Default|GetCurrentRecordTime) (Variables|DataCollection|GetRecordTimeInterval))))

(fn CreateFile
  (params (FileName :type String))
  (bind _returnvalue (Class|EFMBPLibrary|GetGameContentDirectory))
  (bind _datacollectiondirectory (Variables|DataCollection|GetDataCollectionDirectory))
  (bind _returnvalue_2 (Utilities|String|Append _returnvalue _datacollectiondirectory))
  (bind (_bsuccess _newcreatedfile) (Class|EFMBPLibrary|CreateFile _returnvalue_2 FileName))
  (if (Class|BlueprintPathsLibrary|FileExists (Utilities|String|Append _returnvalue_2 FileName))
    (Development|PrintString "File Already Exist!!!!" true true "(R=1.000000,G=0.000000,B=0.000000,A=1.000000)")
    (else
      (if _bsuccess
        _
        (else
          (Development|PrintString "Create File Failed!!!" true true "(R=1.000000,G=0.000000,B=0.000000,A=1.000000)")))
      (return _newcreatedfile))))

(fn RecordPosition
  (bind _character (Variables|DataCollection|GetCharacter))
  ;[1 1 1] Record position in virtual space
  (if (Utilities|IsValid _character)
    (Class|EFMFile|AppendString (Variables|Default|GetVirtualPositionFile) (Utilities|String|ToString(Vector) (Transformation|GetWorldLocation _character)))
    ;[1 1 1] Record position in tracking space
    (Class|EFMFile|AppendString (Variables|Default|GetTrackingPositionFile) (Utilities|String|ToString(Vector) (.OutPosition (Class|SteamVRFunctionLibrary|GetTrackedDevicePositionandOrientation))))))