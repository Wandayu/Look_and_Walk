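; A VR menu actor with two bars that choose between Tutorial and Practice modes.
; When a BP_MotionController overlaps a bar's trigger, that bar switches to an illuminated material, sets its flag and stores the controller; ending the overlap restores the material and clears the flag.
; Tick polls the stored controller's WantsToGrip and opens the tutorial or test level for the flagged bar, with Tutorial taking priority.
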(event OnComponentBeginOverlap(Bar_1)
  (params (OverlappedComponent :type Primitive%20Component%20Object%20Reference) (OtherActor :type Actor%20Object%20Reference) (OtherComp :type Primitive%20Component%20Object%20Reference) (OtherBodyIndex :type Integer) (bFromSweep :type Boolean) (SweepResult :type Hit%20Result%20Structure%20%28by%20ref%29))
  ;[1 1 1] Highlight when Chosen
  ;;[1 1 1] Tutorial Bar Highlight
  (bind _asbp_motion_controller (Utilities|Casting|CastToBP_MotionController OtherActor))
  (Rendering|Material|SetMaterial (Variables|Default|GetBar_1) 0 "/Game/CryoVR_GeneralContent/Materials/M_Illu.M_Illu")
  (Variables|Default|Setis1 true)
  (Variables|Default|SetcurrentController _asbp_motion_controller))

(event OnComponentEndOverlap(Bar_1)
  (params (OverlappedComponent :type Primitive%20Component%20Object%20Reference) (OtherActor :type Actor%20Object%20Reference) (OtherComp :type Primitive%20Component%20Object%20Reference) (OtherBodyIndex :type Integer))
  ;[1 1 1] Highlight when Chosen
  ;;[1 1 1] Tutorial Bar Highlight
  (Utilities|Casting|CastToBP_MotionController OtherActor)
  (Rendering|Material|SetMaterial (Variables|Default|GetBar_1) 0 "/Game/StarterContent/Materials/M_Basic_Wall.M_Basic_Wall")
  (Variables|Default|Setis1 false))

(event OnComponentBeginOverlap(Bar_2)
  (params (OverlappedComponent :type Primitive%20Component%20Object%20Reference) (OtherActor :type Actor%20Object%20Reference) (OtherComp :type Primitive%20Component%20Object%20Reference) (OtherBodyIndex :type Integer) (bFromSweep :type Boolean) (SweepResult :type Hit%20Result%20Structure%20%28by%20ref%29))
  ;[1 1 1] Highlight when Chosen
  ;;[1 1 1] Practice Bar Highlight
  (bind _asbp_motion_controller (Utilities|Casting|CastToBP_MotionController OtherActor))
  (Rendering|Material|SetMaterial (Variables|Default|GetBar_2) 0 "/Game/CryoVR_GeneralContent/Materials/M_Illu.M_Illu")
  (Variables|Default|Setis2 true)
  (Variables|Default|SetcurrentController _asbp_motion_controller))

(event OnComponentEndOverlap(Bar_2)
  (params (OverlappedComponent :type Primitive%20Component%20Object%20Reference) (OtherActor :type Actor%20Object%20Reference) (OtherComp :type Primitive%20Component%20Object%20Reference) (OtherBodyIndex :type Integer))
  ;[1 1 1] Highlight when Chosen
  ;;[1 1 1] Practice Bar Highlight
  (Utilities|Casting|CastToBP_MotionController OtherActor)
  (Rendering|Material|SetMaterial (Variables|Default|GetBar_2) 0 "/Game/StarterContent/Materials/M_Basic_Wall.M_Basic_Wall")
  (Variables|Default|Setis2 false))

(event EventBeginPlay)

(event Collision|EventActorBeginOverlap
  (params (OtherActor :type Actor%20Object%20Reference)))

(event EventTick
  (params (DeltaSeconds :type Float%20%28single-precision%29))
  ;[1 1 1] Game Mode Choice
  ;;[1 1 1] Tutorial Mode
  (if (Variables|Default|Getis1)
    (bind _asbp_motion_controller (Utilities|Casting|CastToBP_MotionController (Variables|Default|GetcurrentController)))
    (if (Variables|/Game/VirtualRealityBP/Blueprints/BP_MotionController.BP_MotionController_C|GetbWantsToGrip _asbp_motion_controller)
      (Game|OpenLevel(byName) (Variables|Default|GetTutorialLevel)))
    (else
      ;;[1 1 1] Practice Mode
      (if (Variables|Default|Getis2)
        (bind _asbp_motion_controller_2 (Utilities|Casting|CastToBP_MotionController (Variables|Default|GetcurrentController)))
        (if (Variables|/Game/VirtualRealityBP/Blueprints/BP_MotionController.BP_MotionController_C|GetbWantsToGrip _asbp_motion_controller_2)
          (Game|OpenLevel(byName) (Variables|Default|GetTest%20Level)))))))

(fn ConstructionScript)