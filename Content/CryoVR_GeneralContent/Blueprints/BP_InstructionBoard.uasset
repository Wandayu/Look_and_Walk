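; BP_InstructionBoard is an in-world board that shows up to three instructions in the CryoVR content.
; SetInstruction converts its three inputs to text and writes them to the text components TR01, TR02 and TR03.
; ClearBoard blanks all three lines.
; The board has no logic of its own in BeginPlay, Tick or construction, so it changes only when these events are called.
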(event Custom|ClearBoard
  ;[1 1 1] Clear all the instructions
  (bind _output_get (Variables|Default|Setdescription ""))
  (Rendering|Components|TextRender|SetText (Variables|Default|GetTR_01) _output_get)
  (Rendering|Components|TextRender|SetText (Variables|Default|GetTR_02) _output_get)
  (Rendering|Components|TextRender|SetText (Variables|Default|GetTR_03) _output_get))

(event Custom|SetInstruction
  (params (Instruction1 :type String) (Instruction2 :type String) (Instruction3 :type String))
  ;[1 1 1] Set the instructions
  (bind _output_get (Variables|Default|Setdescription (Utilities|Text|ToText(String) Instruction1)))
  (Rendering|Components|TextRender|SetText (Variables|Default|GetTR_01) _output_get)
  (bind _output_get_2 (Variables|Default|Setdescription (Utilities|Text|ToText(String) Instruction2)))
  (Rendering|Components|TextRender|SetText (Variables|Default|GetTR_02) _output_get_2)
  (bind _output_get_3 (Variables|Default|Setdescription (Utilities|Text|ToText(String) Instruction3)))
  (Rendering|Components|TextRender|SetText (Variables|Default|GetTR_03) _output_get_3))

(event EventBeginPlay)

(event Collision|EventActorBeginOverlap
  (params (OtherActor :type Actor%20Object%20Reference)))

(event EventTick
  (params (DeltaSeconds :type Float%20%28single-precision%29)))

(fn ConstructionScript)