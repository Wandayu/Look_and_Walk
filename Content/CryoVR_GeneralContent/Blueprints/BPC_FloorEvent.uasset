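; BPC_FloorEvent is a component that returns its parent actor to its starting spot after it touches the floor.
; On BeginPlay it stores the parent's world location and rotation and binds to its begin-overlap event.
; An overlap with a BP_Floor waits for a configurable delay, then teleports the actor back.
; A DoOnce gate, reset a second after the teleport, blocks repeated triggers during the sequence.
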(event Custom|FallonGround
  (params (OverlappedActor :type Actor%20Object%20Reference) (OtherActor :type Actor%20Object%20Reference))
  (Utilities|Casting|CastToBP_Floor OtherActor)
  (Utilities|FlowControl|DoOnce false :!label _label
    (:Completed
      (Utilities|FlowControl|Delay (Variables|Default|GetFloorEventDelay))
      (Transformation|SetActorLocationAndRotation (Variables|Default|GetParentActor) (Variables|Default|GetInitWorldPosition) (Variables|Default|GetInitWorldRotation) false true)
      (Utilities|FlowControl|Delay 1.0)
      (goto _label Reset))))

(event EventBeginPlay
  (bind _parentactor (Variables|Default|GetParentActor))
  (Collision|BindEventtoOnActorBeginOverlap (Variables|Default|GetParentActor) (delegate Custom|FallonGround))
  (Variables|Default|SetInitWorldPosition (Transformation|GetActorLocation _parentactor))
  (Variables|Default|SetInitWorldRotation (Transformation|GetActorRotation _parentactor)))