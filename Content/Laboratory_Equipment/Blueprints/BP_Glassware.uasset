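; BP_Glassware is a configurable laboratory glassware prop that shows one of several beaker, flask, tube, dish or connector meshes filled with coloured liquid.
; The construction script maps the glassware type enum to a static mesh, then creates a dynamic material driven by the liquid colour and amount variables.
; A separate function recolours the liquid with a random pick from a fixed palette; the event graph holds no active logic.
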(event EventBeginPlay)

(event Collision|EventActorBeginOverlap
  (params (OtherActor :type Actor%20Object%20Reference)))

(event EventTick
  (params (DeltaSeconds :type Float%20%28single-precision%29)))

(fn ConstructionScript
  (Components|StaticMesh|SetStaticMesh (Variables|Default|GetStaticMesh) (CallFunction|EGlasswareTypetoSM (Variables|Default|GetGlassware%20Type)))
  (bind _returnvalue (Rendering|Material|CreateDynamicMaterialInstance (Variables|Default|GetStaticMesh) 0 0 "None" :!class /Script/Engine.PrimitiveComponent))
  (Variables|Default|SetGlasswareMaterial _returnvalue)
  (Rendering|Material|SetVectorParameterValue (Variables|Default|GetGlasswareMaterial) "Liquid Colour" (Variables|Default|GetLiquid%20Colour) :!class /Script/Engine.MaterialInstanceDynamic)
  (Rendering|Material|SetScalarParameterValue (Variables|Default|GetGlasswareMaterial) "Liquid Amount" (Variables|Default|GetLiquid%20Amount) :!class /Script/Engine.MaterialInstanceDynamic))

(fn EGlasswareTypetoSM
  (params (Type :type E_Glassware_Type%20Enum :default "NewEnumerator0"))
  (return (Utilities|Select :Index Type :NewEnumerator0 "/Game/Laboratory_Equipment/Meshes/Beaker_500ml.Beaker_500ml" :NewEnumerator1 "/Game/Laboratory_Equipment/Meshes/Beaker_250ml.Beaker_250ml" :NewEnumerator2 "/Game/Laboratory_Equipment/Meshes/Conical_Flask_500ml.Conical_Flask_500ml" :NewEnumerator3 "/Game/Laboratory_Equipment/Meshes/Conical_Flask_250ml.Conical_Flask_250ml" :NewEnumerator4 "/Game/Laboratory_Equipment/Meshes/Flask1.Flask1" :NewEnumerator5 "/Game/Laboratory_Equipment/Meshes/Flask2.Flask2" :NewEnumerator13 "/Game/Laboratory_Equipment/Meshes/Tissue_Culture_Flask.Tissue_Culture_Flask" :NewEnumerator14 "/Game/Laboratory_Equipment/Meshes/Tissue_Culture_Flask_Base.Tissue_Culture_Flask_Base" :NewEnumerator6 "/Game/Laboratory_Equipment/Meshes/Graduated_Cylinder.Graduated_Cylinder" :NewEnumerator12 "/Game/Laboratory_Equipment/Meshes/Test_Tube.Test_Tube" :NewEnumerator11 "/Game/Laboratory_Equipment/Meshes/Petri_Dish.Petri_Dish" :NewEnumerator7 "/Game/Laboratory_Equipment/Meshes/Helix_Connecor_1.Helix_Connecor_1" :NewEnumerator8 "/Game/Laboratory_Equipment/Meshes/Helix_Connector_2.Helix_Connector_2" :NewEnumerator9 "/Game/Laboratory_Equipment/Meshes/Glass_Connecor_1.Glass_Connecor_1" :NewEnumerator10 "/Game/Laboratory_Equipment/Meshes/Glass_Connecor_2.Glass_Connecor_2")))

(fn SetLiquidColour
  (Variables|Default|SetLiquid%20Colour (CallFunction|GetColour))
  (Rendering|Material|SetVectorParameterValue (Variables|Default|GetGlasswareMaterial) "Liquid Colour" (Variables|Default|GetLiquid%20Colour) :!class /Script/Engine.MaterialInstanceDynamic))

(fn GetColour
  (return (Utilities|Select :Index (Math|Random|RandomIntegerinRange 0 11) :Option%200 "(R=0.000000,G=1.000000,B=0.000000,A=1.000000)" :Option%201 "(R=1.000000,G=0.000000,B=0.000000,A=1.000000)" :Option%202 "(R=0.000000,G=0.000000,B=1.000000,A=1.000000)" :Option%203 "(R=1.000000,G=1.000000,B=0.000000,A=1.000000)" :Option%204 "(R=0.700000,G=0.700000,B=0.700000,A=1.000000)" :Option%205 "(R=0.021219,G=0.078187,B=0.000000,A=1.000000)" :Option%206 "(R=0.372000,G=0.000000,B=0.500000,A=1.000000)" :Option%207 "(R=1.000000,G=0.100000,B=0.000000,A=1.000000)" :Option%208 "(R=0.000000,G=1.000000,B=1.000000,A=1.000000)" :Option%209 "(R=1.000000,G=0.000000,B=0.736000,A=1.000000)" :Option%2010 "(R=0.000000,G=0.000000,B=0.000000,A=1.000000)")))