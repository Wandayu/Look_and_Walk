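; BP_LabBottle is a configurable lab glassware prop covering bottles, flasks and a petri dish.
; The construction script picks the mesh by bottle type and creates dynamic materials for bottle (glass or plastic, with or without label) and hideable cap.
; It then applies colors, label, liquid level and glow.
; Helper functions set default or random labels and random colors, flagging full-color label textures through set membership.
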(event EventBeginPlay)

(event Collision|EventActorBeginOverlap
  (params (OtherActor :type Actor%20Object%20Reference)))

(event EventTick
  (params (DeltaSeconds :type Float%20%28single-precision%29)))

(fn ConstructionScript
  ;[0 1 0.3093] Set Static mesh to E_Bottletype from Defaults
  (Components|StaticMesh|SetStaticMesh (Variables|Default|GetStaticMesh) (CallFunction|ELabBottleTypetoSM (Variables|Default|GetBottle%20Type)))
  ;[0.7059 1 0] Create a Dynamic Material Instance for the Cap
  (bind _returnvalue (Rendering|Material|CreateDynamicMaterialInstance (Variables|Default|GetStaticMesh) 1 (select (Variables|Default|GetHide%20Cap) "/Game/LabBottles/Materials/M_Hidden.M_Hidden" "/Game/LabBottles/Materials/M_BottleCaps.M_BottleCaps") :!class /Script/Engine.PrimitiveComponent))
  (Variables|Default|SetCapMat _returnvalue)
  ;[1 0.652 0] Create a Dynamic Material Instance for the Bottle
  (bind _returnvalue_2 (Rendering|Material|CreateDynamicMaterialInstance (Variables|Default|GetStaticMesh) 0 (select (Variables|Default|GetGlass) (select (Variables|Default|GetHas%20Lable) "/Game/LabBottles/Materials/M_GlassBottles.M_GlassBottles" "/Game/LabBottles/Materials/MI_GlassNoLable.MI_GlassNoLable") (select (Variables|Default|GetHas%20Lable) "/Game/LabBottles/Materials/M_PlasticBottles.M_PlasticBottles" "/Game/LabBottles/Materials/Mi_PlasticNoLable.Mi_PlasticNoLable")) :!class /Script/Engine.PrimitiveComponent))
  (Variables|Default|SetBottleMat _returnvalue_2)
  ;[0.8914 0 1] sets Parameters in the Material Instance
  ; -the Lable Texture from the Defaults
  ; -Single Color Lable or not
  (CallFunction|SetLableParameter)
  ;[0 0.8986 1] Sets Parameters From Defaults to Material Instance
  (Rendering|Material|SetVectorParameterValue (Variables|Default|GetBottleMat) "Base Color" (Variables|Default|GetBase%20Color) :!class /Script/Engine.MaterialInstanceDynamic)
  (Rendering|Material|SetVectorParameterValue (Variables|Default|GetCapMat) "Base Color" (Variables|Default|GetCapColor) :!class /Script/Engine.MaterialInstanceDynamic)
  (Rendering|Material|SetVectorParameterValue (Variables|Default|GetBottleMat) "Lable Color" (Variables|Default|GetLable%20Color) :!class /Script/Engine.MaterialInstanceDynamic)
  (Rendering|Material|SetScalarParameterValue (Variables|Default|GetBottleMat) "Liquid Level" (Variables|Default|GetLiquid%20Level) :!class /Script/Engine.MaterialInstanceDynamic)
  (Rendering|Material|SetScalarParameterValue (Variables|Default|GetBottleMat) "Liquid Glow" (Variables|Default|GetGlow) :!class /Script/Engine.MaterialInstanceDynamic))

(fn ELabBottleTypetoSM
  (params (Type :type E_LabBottleType%20Enum :default "NewEnumerator0"))
  (return (Utilities|Select :Index Type :NewEnumerator0 "/Game/LabBottles/Meshes/MediaBottles/SM_MediaBottle_100ml.SM_MediaBottle_100ml" :NewEnumerator1 "/Game/LabBottles/Meshes/MediaBottles/SM_MediaBottle_250ml.SM_MediaBottle_250ml" :NewEnumerator2 "/Game/LabBottles/Meshes/MediaBottles/SM_MediaBottle_500ml.SM_MediaBottle_500ml" :NewEnumerator3 "/Game/LabBottles/Meshes/MediaBottles/SM_MediaBottle_1000ml.SM_MediaBottle_1000ml" :NewEnumerator4 "/Game/LabBottles/Meshes/MediaBottles/SM_MediaBottle_2000ml.SM_MediaBottle_2000ml" :NewEnumerator5 "/Game/LabBottles/Meshes/MediaBottles/SM_MediaBottle_5000ml.SM_MediaBottle_5000ml" :NewEnumerator6 "/Game/LabBottles/Meshes/MediaBottles/SM_MediaBottle_10000ml.SM_MediaBottle_10000ml" :NewEnumerator7 "/Game/LabBottles/Meshes/Miscellaneous/SM_Bottel_Rec_1.SM_Bottel_Rec_1" :NewEnumerator8 "/Game/LabBottles/Meshes/Miscellaneous/SM_Bottel_Rec_2.SM_Bottel_Rec_2" :NewEnumerator9 "/Game/LabBottles/Meshes/Miscellaneous/SM_Bottel_Rec_3.SM_Bottel_Rec_3" :NewEnumerator10 "/Game/LabBottles/Meshes/Miscellaneous/SM_Bottle_Small.SM_Bottle_Small" :NewEnumerator11 "/Game/LabBottles/Meshes/Miscellaneous/SM_Bottle_middle.SM_Bottle_middle" :NewEnumerator12 "/Game/LabBottles/Meshes/Miscellaneous/SM_Bottle_big.SM_Bottle_big" :NewEnumerator13 "/Game/LabBottles/Meshes/Miscellaneous/SM_Bottle_Handle.SM_Bottle_Handle" :NewEnumerator14 "/Game/LabBottles/Meshes/Miscellaneous/SM_ErlenmeyerFlask.SM_ErlenmeyerFlask" :NewEnumerator15 "/Game/LabBottles/Meshes/Miscellaneous/SM_GraduateFlask.SM_GraduateFlask" :NewEnumerator16 "/Game/LabBottles/Meshes/Miscellaneous/SM_MeasuringFlask.SM_MeasuringFlask" :NewEnumerator17 "/Game/LabBottles/Meshes/Miscellaneous/SM_PetriDish.SM_PetriDish" :NewEnumerator18 "/Game/LabBottles/Meshes/Miscellaneous/SM_RoundFlask.SM_RoundFlask")))

(fn SetDefaultLable
  ;[0.7767 1 0.06994] sets Lable to the Specified Default
  (Variables|Default|SetLable (Utilities|Select :Index (Variables|Default|GetBottle%20Type) :NewEnumerator0 "/Game/LabBottles/Textures/T_Metric_100ml.T_Metric_100ml" :NewEnumerator1 "/Game/LabBottles/Textures/T_Metric_250ml.T_Metric_250ml" :NewEnumerator2 "/Game/LabBottles/Textures/T_Metric_500ml.T_Metric_500ml" :NewEnumerator3 "/Game/LabBottles/Textures/T_Metric_1000ml.T_Metric_1000ml" :NewEnumerator4 "/Game/LabBottles/Textures/T_Metric_2000ml.T_Metric_2000ml" :NewEnumerator5 "/Game/LabBottles/Textures/T_Metric_5000ml.T_Metric_5000ml" :NewEnumerator6 "/Game/LabBottles/Textures/T_Metric_10000ml.T_Metric_10000ml" :NewEnumerator7 "/Game/LabBottles/Textures/T_Sign01_Text01.T_Sign01_Text01" :NewEnumerator8 "/Game/LabBottles/Textures/T_Sign02_Ethanol.T_Sign02_Ethanol" :NewEnumerator9 "/Game/LabBottles/Textures/T_Sign03_Copper.T_Sign03_Copper" :NewEnumerator10 "/Game/LabBottles/Textures/T_Sign04_Iodine.T_Sign04_Iodine" :NewEnumerator11 "/Game/LabBottles/Textures/T_Sign05_NFPA_Rating01.T_Sign05_NFPA_Rating01" :NewEnumerator12 "/Game/LabBottles/Textures/T_Sign06_NFPA_Rating02.T_Sign06_NFPA_Rating02" :NewEnumerator13 "/Game/LabBottles/Textures/T_Sign07_NFPA_Rating03.T_Sign07_NFPA_Rating03" :NewEnumerator14 "/Game/LabBottles/Textures/T_Metric_Alpha.T_Metric_Alpha" :NewEnumerator15 "/Game/LabBottles/Textures/T_Metric_Alpha.T_Metric_Alpha" :NewEnumerator16 "/Game/LabBottles/Textures/T_Metric_Alpha.T_Metric_Alpha" :NewEnumerator17 0 :NewEnumerator18 "/Game/LabBottles/Textures/T_Metric_Alpha.T_Metric_Alpha"))
  ;[0.8914 0 1] sets Parameters in the Material Instance
  ; -the Label Texture from the Defaults
  ; -Single Color Lable or not
  (CallFunction|SetLableParameter))

(fn GetRandomLable
  ;[0 1 0.5489] Combines Both sets of Lable Types and Returns a Random entry of the Combined Set
  (bind _result (Utilities|Set|Union (Variables|LabelsTochoosefrom|GetSingle%20Color%20Lables) (Variables|LabelsTochoosefrom|GetColor%20Lables)))
  (bind _result_2 (Utilities|Set|ToArray _result))
  (return (Utilities|Array|Get(acopy) _result_2 (Math|Random|RandomIntegerinRange 0 (Utilities|Array|Length _result_2)))))

(fn SetRandomLable
  (Variables|Default|SetLable (CallFunction|GetRandomLable))
  ;[0.8914 0 1] sets Parameters in the Material Instance
  ; -the Lable Texture from the Defaults
  ; -Single Color Lable or not
  (CallFunction|SetLableParameter))

(fn SetRandomBaseColor
  (Variables|Default|SetBase%20Color (CallFunction|GetRandomColor))
  (Rendering|Material|SetVectorParameterValue (Variables|Default|GetBottleMat) "Base Color" (Variables|Default|GetBase%20Color) :!class /Script/Engine.MaterialInstanceDynamic))

(fn SetRandomCapColor
  (Variables|Default|SetCapColor (CallFunction|GetRandomColor))
  (Rendering|Material|SetVectorParameterValue (Variables|Default|GetCapMat) "Base Color" (Variables|Default|GetCapColor) :!class /Script/Engine.MaterialInstanceDynamic))

(fn GetRandomColor
  (return (Utilities|Select :Index (Math|Random|RandomIntegerinRange 0 7) :Option%200 "(R=1.000000,G=0.049471,B=0.000000,A=1.000000)" :Option%201 "(R=1.000000,G=0.000000,B=0.000000,A=1.000000)" :Option%202 "(R=0.000000,G=0.250000,B=1.000000,A=1.000000)" :Option%203 "(R=1.000000,G=0.431106,B=0.000000,A=1.000000)" :Option%204 "(R=0.101769,G=0.656250,B=0.000000,A=1.000000)" :Option%205 "(R=0.836623,G=0.000000,B=0.854167,A=1.000000)" :Option%206 "(R=0.700000,G=0.700000,B=0.700000,A=1.000000)" :Option%207 "(R=0.000000,G=0.000000,B=0.000000,A=1.000000)")))

(fn SetRandomLableColor
  (Variables|Default|SetLable%20Color (CallFunction|GetRandomColor))
  (Rendering|Material|SetVectorParameterValue (Variables|Default|GetBottleMat) "Lable Color" (Variables|Default|GetLable%20Color) :!class /Script/Engine.MaterialInstanceDynamic))

(fn SetLableParameter
  (Rendering|Material|SetScalarParameterValue (Variables|Default|GetBottleMat) "Colored Lable" (Math|Conversions|ToFloat(Boolean) (Utilities|Set|Contains (Variables|LabelsTochoosefrom|GetColor%20Lables) (Variables|Default|GetLable))) :!class /Script/Engine.MaterialInstanceDynamic)
  (Rendering|Material|SetTextureParameterValue (Variables|Default|GetBottleMat) "Lable" (Variables|Default|GetLable)))